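; Pressure switch Blueprint that changes its switch state when something begins overlapping its trigger box.
; The overlap calls ChangeSwitchState on a Switchable component with no actor filter or end-overlap handling.
; The component's SwitchEvent brightens or dims the mesh through an intensity material parameter.
; The construction script creates a dynamic instance of the emissive material on the mesh's second material slot.
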(event `self.Box.OnComponentBeginOverlap`
  (params (OverlappedComponent :type "PrimitiveComponent Object Reference") (OtherActor :type "Actor Object Reference") (OtherComp :type "PrimitiveComponent Object Reference") (OtherBodyIndex :type Integer) (bFromSweep :type Boolean) (SweepResult :type "HitResult Structure (by ref)"))
  (`Switchable.ChangeSwitchState` (`self.Switchable`)))

(event `self.Switchable.SwitchEvent`
  (params (SwitchingActor :type "Actor Object Reference") (SwitchState :type Boolean))
  (bind _staticmeshcomponent (`self.StaticMeshComponent`))
  (if SwitchState
    (`MeshComponent.SetScalarParameterValueOnMaterials` _staticmeshcomponent "Intensety" 1.0)
    (else
      (`MeshComponent.SetScalarParameterValueOnMaterials` _staticmeshcomponent "Intensety" 0.1))))

(fn `UserConstructionScript`
  (bind _returnvalue (`PrimitiveComponent.CreateDynamicMaterialInstance` (`self.StaticMeshComponent`) 1 "/Game/Assets/Material/EmissiveMat.EmissiveMat"))
  (set `self.DynamicMaterial` _returnvalue))